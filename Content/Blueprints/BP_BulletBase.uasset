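; BP_BulletBase is a bullet actor that resolves its impact when its collision component hits something.
; A hit on its owner only destroys the bullet.
; Any other hit applies fixed damage, spawns an impact emitter selected by surface type, and attaches a short-lived dirt decal aligned to the hit normal.
; Physics-simulating components also receive a velocity-scaled impulse before the bullet destroys itself.
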(event OnComponentHit(BulletCollision)
  (params (HitComponent :type Primitive%20Component%20Object%20Reference) (OtherActor :type Actor%20Object%20Reference) (OtherComp :type Primitive%20Component%20Object%20Reference) (NormalImpulse :type Vector :default "0, 0, 0") (Hit :type Hit%20Result%20Structure%20%28by%20ref%29))
  (bind _returnvalue (Components|GetOwner))
  (bind (_bblockinghit _binitialoverlap _time _distance _location _impactpoint _normal) (Collision|BreakHitResult Hit))
  (bind _returnvalue_2 (Math|Conversions|RotationFromXVector _normal))
  (if (== OtherActor _returnvalue)
    (Actor|DestroyActor)
    (else
      (Game|Damage|ApplyDamage OtherActor 5.0 0 _returnvalue)
      (Effects|SpawnEmitteratLocation (Utilities|Select :Index (Collision|GetSurfaceType Hit) :SurfaceType_Default "/Game/GKnight/Art/Effects/Particles/PS_Impact_Bullet_Concrete.PS_Impact_Bullet_Concrete") _location _returnvalue_2)
      (Class|GameplayStatics|SpawnDecalAttached "/Game/GKnight/Art/Effects/Materials/MI_Decal_Bullet_Dirt.MI_Decal_Bullet_Dirt" "6.000000,6.000000,6.000000" OtherComp "None" _location _returnvalue_2 "KeepWorldPosition" 5.0)
      (if (Physics|IsSimulatingPhysics OtherComp "None")
        (Physics|AddImpulse OtherComp (* (Transformation|GetVelocity) 0.01) "None" true))
      (Utilities|IsValid self
        (:Is%20Valid
          (Actor|DestroyActor))))))

(event EventBeginPlay)

(event Collision|EventActorBeginOverlap
  (params (OtherActor :type Actor%20Object%20Reference)))

(fn ConstructionScript)